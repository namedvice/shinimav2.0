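; BP_Skins is a data-driven character skin Blueprint that sets up a skeletal mesh, particles and an optional shield.
; The construction script looks up RowName in DT_Skins and copies visual, socket, speed and score-multiplier data into variables.
; BeginPlay applies the mesh, attaches the emitter without checking HaveParticles, and attaches the shield mesh when Shield is set.
; Material, Speed and ScoreX2 are only stored here.
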(event `self.ReceiveBeginPlay`
  (bind _skeletalmesh (`self.SkeletalMesh`))
  (bind _shieldmesh (`self.ShieldMesh`))
  (bind _skeletalmesh_2 (`self.SkeletalMesh`))
  (`SkinnedMeshComponent.SetSkinnedAssetAndUpdate` _skeletalmesh (`self.Skin`) true)
  (`GameplayStatics.SpawnEmitterAttached` (`self.Particles`) _skeletalmesh (`SkinnedMeshComponent.GetSocketBoneName` _skeletalmesh (`self.Socket Particles`)))
  (if (`self.Shield`)
    (`StaticMeshComponent.SetStaticMesh` _shieldmesh (`self.Shield Mesh`))
    (`SceneComponent.K2_AttachToComponent` _shieldmesh _skeletalmesh_2 (`SkinnedMeshComponent.GetSocketBoneName` _skeletalmesh_2 (`self.Socket Shield`)) "KeepRelative" "KeepRelative" "KeepRelative" true)))

(fn `UserConstructionScript`
  (bind _returnvalue (`|GetDataTableRow` "/Game/ShinimaSecVer/Data/DT_Skins.DT_Skins" (`self.RowName`))
    (:`then`
      (bind _output_get (set `self.RowSkinsData` _returnvalue))
      (bind (_skin _speed _shield _shieldmesh _socketshield _material _socketparticles _haveparticles _particles _scoremultiply) (break `/Game/ShinimaSecVer/Data/SSkins` _output_get))
      (set `self.Skin` _skin)
      (set `self.Speed` _speed)
      (set `self.Shield` _shield)
      (set `self.Shield Mesh` _shieldmesh)
      (set `self.Material` _material)
      (set `self.Socket Shield` _socketshield)
      (set `self.Socket Particles` _socketparticles)
      (set `self.Have Particles` _haveparticles)
      (set `self.Particles` _particles)
      (set `self.Score X2` _scoremultiply))))