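; Generator actor that periodically spawns BP_Column actors into the level.
; On BeginPlay it spawns one column far ahead along world X and another at the ColumnLocation component, then repeats the latter spawn on a looping timer.
; A disconnected, never-run loop would spawn weighted-random obstacles, shields and rate-limited arcs, using FindSpawnPosition to re-roll points already overlapped by obstacles.
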(event `self.ReceiveBeginPlay`
  (bind _returnvalue_location (`KismetMathLibrary.BreakTransform` (`self.GetTransform`)))
  (`|SpawnActorFromClass` "/Game/ShinimaSecVer/Core/ObstaclesGenerator/BP_Column.BP_Column_C" (`KismetMathLibrary.MakeTransform` (+ _returnvalue_location (80000.0 0.0 0.0))) "AlwaysSpawn" "OverrideRootScale" null null)
  (`self.SpawnColumns`)
  (`KismetSystemLibrary.K2_SetTimerDelegate` (delegate `SpawnColumns`) 120.0 true))

(event `SpawnColumns`
  (`|SpawnActorFromClass` "/Game/ShinimaSecVer/Core/ObstaclesGenerator/BP_Column.BP_Column_C" (`SceneComponent.K2_GetComponentToWorld` (`self.ColumnLocation`)) "AlwaysSpawn" "OverrideRootScale" null null))

(fn `FindSpawnPosition`
  (returns (OutItem :type "SceneComponent Object Reference"))
  (locals (LSpawnPositions :type "Array of SceneComponent Object Reference") (LRandomIndex :type Integer :default 0))
  (bind _array (`|MakeArray` null null null null null null null :!type "SceneComponent Object Reference"))
  (bind _lspawnpositions (`local.LSpawnPositions`))
  (bind _output (`|GetArrayItem` _lspawnpositions (`local.LRandomIndex`)))
  (set `local.LSpawnPositions` _array)
  (bind _output_get (set `local.LRandomIndex` (`.OutIndex` (`KismetArrayLibrary.Array_Random` _array)) :!label _label))
  (bind (_outactors _returnvalue) (`KismetSystemLibrary.BoxOverlapActors` (`SceneComponent.K2_GetComponentLocation` (`|GetArrayItem` (`local.LSpawnPositions`) _output_get)) (10.0 10.0 10.0) (`|MakeArray` "ObjectTypeQuery1" "ObjectTypeQuery2" :!type "EObjectTypeQuery Enum") "/Game/ShinimaSecVer/Core/ObstaclesGenerator/BP_ObstacleBase.BP_ObstacleBase_C" (`|MakeArray` self :!type "Actor Object Reference")))
  (if _returnvalue
    (`KismetArrayLibrary.Array_RemoveItem` _lspawnpositions _output)
    (`KismetSystemLibrary.PrintString` "Fuck!")
    (goto _label)
    (else
      (return _output))))

(fn `UserConstructionScript`)