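; BP_BlockingWalls is a soft barrier actor that pushes the player out along its forward vector.
; Entering its Box starts a looping fast timer that adds velocity-change impulses to the player's character movement; leaving clears it.
; Push strength is inversely proportional to the player's local X distance from the Box's relative location, so it grows sharply as the player nears the box's center plane.
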(event `self.Box.OnComponentBeginOverlap`
  (params (OverlappedComponent :type "PrimitiveComponent Object Reference") (OtherActor :type "Actor Object Reference") (OtherComp :type "PrimitiveComponent Object Reference") (OtherBodyIndex :type Integer) (bFromSweep :type Boolean) (SweepResult :type "HitResult Structure (by ref)"))
  (if (== OtherActor (`GameplayStatics.GetPlayerCharacter` 0))
    (bind _returnvalue (`KismetSystemLibrary.K2_SetTimerDelegate` (delegate `PushCharacterOut`) 0.01 true))))

(event `PushCharacterOut`
  (bind _returnvalue (`GameplayStatics.GetPlayerCharacter` 0))
  (bind _returnvalue_x (`KismetMathLibrary.BreakVector` (`KismetMathLibrary.InverseTransformLocation` (`self.GetTransform`) (`self.K2_GetActorLocation` _returnvalue))))
  (`CharacterMovementComponent.AddImpulse` (`Character.CharacterMovement` _returnvalue) (* (`self.GetActorForwardVector`) (* (/ 1.0 (`KismetMathLibrary.Abs` (- (.x (`SceneComponent.RelativeLocation` (`self.Box`))) _returnvalue_x))) 5000.0)) true))

(event `self.Box.OnComponentEndOverlap`
  (params (OverlappedComponent :type "PrimitiveComponent Object Reference") (OtherActor :type "Actor Object Reference") (OtherComp :type "PrimitiveComponent Object Reference") (OtherBodyIndex :type Integer))
  (if (== OtherActor (`GameplayStatics.GetPlayerCharacter` 0))
    (`KismetSystemLibrary.K2_ClearAndInvalidateTimerHandle` (stale `self.Box.OnComponentBeginOverlap` _returnvalue))))

(fn `UserConstructionScript`)