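; Road tile actor that randomizes its look on BeginPlay, picking one mesh each from StartMeshes and AfterStartMeshes.
; When the player enters its Box, it calls RoadTile on GM_Base, then destroys itself after a delay.
; GetAttachTransform exposes the Arrow's world transform as an attach point, likely for chaining tiles.
; Overlaps on the first mesh component call ApplyDamage on the other actor.
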(event `self.ReceiveBeginPlay`
  (`StaticMeshComponent.SetStaticMesh` (`self.StaticMesh`) (`KismetArrayLibrary.Array_Random` (`self.StartMeshes`)))
  (`StaticMeshComponent.SetStaticMesh` (`self.SecondMesh`) (`KismetArrayLibrary.Array_Random` (`self.AfterStartMeshes`))))

(event `self.Box.OnComponentBeginOverlap`
  (params (OverlappedComponent :type "PrimitiveComponent Object Reference") (OtherActor :type "Actor Object Reference") (OtherComp :type "PrimitiveComponent Object Reference") (OtherBodyIndex :type Integer) (bFromSweep :type Boolean) (SweepResult :type "HitResult Structure (by ref)"))
  (if (== OtherActor (`GameplayStatics.GetPlayerCharacter` 0))
    (bind _asgm_base (cast `/Game/ShinimaSecVer/Core/GameModes/GM_Base` (`GameplayStatics.GetGameMode`)))
    (`/Game/ShinimaSecVer/Core/GameModes/GM_Base.RoadTile` _asgm_base)
    (`KismetSystemLibrary.Delay` 10.0)
    (`self.K2_DestroyActor`)))

(event `self.StaticMesh.OnComponentBeginOverlap`
  (params (OverlappedComponent :type "PrimitiveComponent Object Reference") (OtherActor :type "Actor Object Reference") (OtherComp :type "PrimitiveComponent Object Reference") (OtherBodyIndex :type Integer) (bFromSweep :type Boolean) (SweepResult :type "HitResult Structure (by ref)"))
  (`GameplayStatics.ApplyDamage` OtherActor 0.0 null self))

(fn `GetAttachTransform`
  (returns (WorldTransform :type "Transform Structure"))
  (return (`SceneComponent.K2_GetComponentToWorld` (`self.Arrow`))))

(fn `UserConstructionScript`)