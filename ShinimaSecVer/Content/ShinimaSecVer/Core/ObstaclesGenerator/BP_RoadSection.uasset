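; BP_RoadSection is a road segment actor, apparently for an obstacle generator, that randomizes its look and can damage actors.
; Initialize sets the static mesh to a random entry from its segment list.
; Its Sphere component applies fixed damage to whatever hits it.
; Socket-based placement of random obstacle meshes with random 90-degree turns is present but disconnected and never runs, as is a left/right obstacle pick by socket name.
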(event `Initialize`
  (`StaticMeshComponent.SetStaticMesh` (`self.StaticMesh`) (`KismetArrayLibrary.Array_Random` (`self.RoadSegmets`))))

(event `self.ReceiveBeginPlay`)

(event `self.Sphere.OnComponentHit`
  (params (HitComponent :type "PrimitiveComponent Object Reference") (OtherActor :type "Actor Object Reference") (OtherComp :type "PrimitiveComponent Object Reference") (NormalImpulse :type "Vector Structure") (Hit :type "HitResult Structure (by ref)"))
  (`GameplayStatics.ApplyDamage` OtherActor 10.0))

(fn `UserConstructionScript`)