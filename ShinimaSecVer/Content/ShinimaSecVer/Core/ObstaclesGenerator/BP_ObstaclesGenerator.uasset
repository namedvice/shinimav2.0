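; BP_ObstaclesGenerator is an obstacle spawner actor that places BP_Column actors in the level over time.
; On BeginPlay it spawns one column far ahead of itself along world X, then starts a looping one-minute timer.
; Each timer tick spawns another column at the Scene4 component's transform.
; A delayed loop that spawns BP_Obstacle at one of four random scene points is present but disconnected, so it never runs.
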(event `self.ReceiveBeginPlay`
  (bind _returnvalue_location (`KismetMathLibrary.BreakTransform` (`self.GetTransform`)))
  (`|SpawnActorFromClass` "/Game/ShinimaSecVer/Core/ObstaclesGenerator/BP_Column.BP_Column_C" (`KismetMathLibrary.MakeTransform` (+ _returnvalue_location (80000.0 0.0 0.0))) "AlwaysSpawn" "OverrideRootScale" null null)
  (`KismetSystemLibrary.K2_SetTimerDelegate` (delegate `SpawnColumns`) 60.0 true))

(event `SpawnColumns`
  (`|SpawnActorFromClass` "/Game/ShinimaSecVer/Core/ObstaclesGenerator/BP_Column.BP_Column_C" (`SceneComponent.K2_GetComponentToWorld` (`self.Scene4`)) "AlwaysSpawn" "OverrideRootScale" null null))

(fn `UserConstructionScript`)