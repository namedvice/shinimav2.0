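; Base obstacle actor that damages whatever it hits and destroys itself after DeathTime.
; On BeginPlay it picks a random mesh for the Sphere component and attaches a particle emitter at every mesh socket, using socket X and Y scale.
; Roughly one in ten obstacles also rotates on all axes through a timeline.
; A hit applies fixed damage and disables the Sphere's collision.
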(event `self.ReceiveBeginPlay`
  (bind _sphere (`self.Sphere`))
  (bind _sphere_2 (`self.Sphere`))
  (`StaticMeshComponent.SetStaticMesh` (`self.Sphere`) (`KismetArrayLibrary.Array_Random` (`self.New Mesh`)))
  (if (<= (`KismetMathLibrary.RandomIntegerInRange` 0 100) 10)
    (`self.Rotative`))
  (for _array_element (`SceneComponent.GetAllSocketNames` _sphere)
    (bind _returnvalue (`SceneComponent.GetSocketTransform` _sphere_2 _array_element "RTS_Actor"))
    ;[1 1 1] For Obstacle Particles
    (`GameplayStatics.SpawnEmitterAttached` "/Game/ShinimaSecVer/VFX/PS_Triag.PS_Triag" (`self.Sphere`) "None" (`SceneComponent.GetSocketLocation` _sphere _array_element) (`SceneComponent.GetSocketRotation` _sphere_2 _array_element) (`KismetMathLibrary.MakeVector` (.x (.scale _returnvalue)) (.y (.scale _returnvalue)) 1.0) "KeepWorldPosition"))
  (`KismetSystemLibrary.Delay` (`self.DeathTime`))
  (`self.K2_DestroyActor`))

(event `self.Sphere.OnComponentHit`
  (params (HitComponent :type "PrimitiveComponent Object Reference") (OtherActor :type "Actor Object Reference") (OtherComp :type "PrimitiveComponent Object Reference") (NormalImpulse :type "Vector Structure") (Hit :type "HitResult Structure (by ref)"))
  (`GameplayStatics.ApplyDamage` OtherActor 10.0 null self)
  (`PrimitiveComponent.SetCollisionEnabled` (`self.Sphere`) "NoCollision"))

(event `Rotative`
  (bind _sphere (`self.Sphere`))
  (bind (_direction _newtrack_0) (`Timeline|Timeline_0`)
    (:`Update`
      (`/Engine/EditorBlueprintResources/StandardMacros.IsValid` _sphere
        (:`Is Valid`
          (`SceneComponent.K2_SetWorldRotation` _sphere (`KismetMathLibrary.MakeRotator` _newtrack_0 _newtrack_0 _newtrack_0) false false))))))

(event `self.ReceiveAnyDamage`
  (params (Damage :type "Float (single-precision)") (DamageType :type "DamageType Object Reference") (InstigatedBy :type "Controller Object Reference") (DamageCauser :type "Actor Object Reference")))

(fn `UserConstructionScript`)