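; BP_Shop is a shop actor whose box trigger halts the player's flying and switches the character to an idle pose.
; BeginPlay caches the player as BP_PlayerCharacter.
; Box overlap sets MaxFlySpeed to zero and plays a non-looping idle in single-node animation mode; leaving restores a fixed speed and Animation Blueprint mode.
; Overlap handlers never check the overlapping actor, and no purchase logic exists here.
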(event `self.ReceiveBeginPlay`
  (bind _asbp_player_character (cast `/Game/ShinimaSecVer/Core/Characters/BP_PlayerCharacter` (`GameplayStatics.GetPlayerPawn` 0)))
  (set `self.As BP Player Character` _asbp_player_character))

(event `self.Box.OnComponentBeginOverlap`
  (params (OverlappedComponent :type "PrimitiveComponent Object Reference") (OtherActor :type "Actor Object Reference") (OtherComp :type "PrimitiveComponent Object Reference") (OtherBodyIndex :type Integer) (bFromSweep :type Boolean) (SweepResult :type "HitResult Structure (by ref)"))
  (bind _as_bp_player_character (`self.As BP Player Character`)
    (:`then`
      (set `CharacterMovementComponent.MaxFlySpeed` 0.0 (`Character.CharacterMovement` _as_bp_player_character))
      (bind _mesh (`Character.Mesh` _as_bp_player_character))
      (`SkeletalMeshComponent.SetAnimationMode` _mesh "AnimationSingleNode")
      (`SkeletalMeshComponent.PlayAnimation` _mesh "/Game/Mannequin/Animations/ThirdPersonIdle.ThirdPersonIdle" false))
    (:`else`)))

(event `self.Box.OnComponentEndOverlap`
  (params (OverlappedComponent :type "PrimitiveComponent Object Reference") (OtherActor :type "Actor Object Reference") (OtherComp :type "PrimitiveComponent Object Reference") (OtherBodyIndex :type Integer))
  (bind _as_bp_player_character (`self.As BP Player Character`)
    (:`then`
      (set `CharacterMovementComponent.MaxFlySpeed` 1200.0 (`Character.CharacterMovement` _as_bp_player_character))
      (bind _mesh (`Character.Mesh` _as_bp_player_character))
      (`SkeletalMeshComponent.SetAnimationMode` _mesh "AnimationBlueprint")
      (`SkeletalMeshComponent.LinkAnimClassLayers` _mesh "/Game/Mannequin/Animations/ThirdPerson_AnimBP.ThirdPerson_AnimBP_C"))
    (:`else`)))

(fn `UserConstructionScript`)