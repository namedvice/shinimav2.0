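; Base game mode that lays out the opening stretch of road when play begins by spawning five chained tiles.
; Each RoadTile call spawns a BP_Column and a BP_SpawnerRoads at the stored SpawnTransform, then drops the road by a fixed Z offset.
; The road's attach transform, raised back by that offset, becomes the next SpawnTransform, so each tile continues from the previous one.
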(event `self.ReceiveBeginPlay`
  (for _ (range 5)
    (`self.RoadTile`)))

(fn `RoadTile`
  (bind (_spawn_transform_location _spawn_transform_rotation) (`KismetMathLibrary.BreakTransform` (`self.Spawn Transform`)))
  (`|SpawnActorFromClass` "/Game/ShinimaSecVer/Core/ObstaclesGenerator/BP_Column.BP_Column_C" (`KismetMathLibrary.MakeTransform` _spawn_transform_location _spawn_transform_rotation) "Undefined" "OverrideRootScale" null null)
  (bind _returnvalue (`|SpawnActorFromClass` "/Game/ShinimaSecVer/Core/ObstaclesGenerator/BP_SpawnerRoads.BP_SpawnerRoads_C" (`self.Spawn Transform`) "Undefined" "OverrideRootScale" null null))
  (`self.K2_AddActorWorldOffset` _returnvalue (0.0 0.0 -700.0) false false)
  (bind _worldtransform (`/Game/ShinimaSecVer/Core/ObstaclesGenerator/BP_SpawnerRoads.GetAttachTransform` _returnvalue))
  (set `self.Spawn Transform` (`KismetMathLibrary.MakeTransform` (`KismetMathLibrary.MakeVector` (.x (.location _worldtransform)) (.y (.location _worldtransform)) (+ (.z (.location _worldtransform)) 700.0)) (.rotation _worldtransform) (.scale _worldtransform))))

(fn `UserConstructionScript`)