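; Cube Runner map-generation Blueprint that builds randomized background scenery from tall instanced meshes set far below the origin.
; CreateMapBackground clears its Hierarchical Instanced Static Mesh, then fills a jittered grid, randomly skipping some cells and varying footprint and height.
; X spacing is re-rolled per instance, and LastX is set from the final column index with a fresh random spacing after the loops.
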(event `CreateMapBackground`
  (params (LastX :type Integer))
  (bind _randomscale (`self.RandomScale`))
  ;[0.05382 0.05382 0.05382] Map Background
  (`InstancedStaticMeshComponent.ClearInstances` (`self.HierarchicalInstancedStaticMesh_Background1`))
  (for _index (range 12)
    (for _index_2 (range 71)
      (if (`KismetMathLibrary.RandomBoolWithWeight` 0.8)
        (set `self.RandomScale` (`KismetMathLibrary.RandomFloatInRange` 22.0 44.0))
        (bind _returnvalue (* _index_2 (`KismetMathLibrary.RandomIntegerInRange` 4000 5000)))
        (`InstancedStaticMeshComponent.AddInstance` (`self.HierarchicalInstancedStaticMesh_Background1`) (`KismetMathLibrary.MakeTransform` (`KismetMathLibrary.MakeVector` (`KismetMathLibrary.Conv_IntToDouble` _returnvalue) (`KismetMathLibrary.Conv_IntToDouble` (- (* _index 7000) 41000)) -60100.0) (struct) (`KismetMathLibrary.MakeVector` _randomscale _randomscale (`KismetMathLibrary.Conv_IntToDouble` (`KismetMathLibrary.RandomIntegerInRange` 1000 1200))))))))
  (set `self.LastX` _returnvalue))

(fn `UserConstructionScript`)