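; BP_BlockingWalls is a soft barrier actor that pushes the player character along the wall's forward vector while they overlap its Box.
; Overlap begin starts a fast looping timer, and overlap end clears it.
; Each timer tick zeroes the player's Y and Z velocity, then applies a velocity-change impulse inversely proportional to the local X distance from the Box.
; It also prints that distance for debugging.
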(event `self.Box.OnComponentBeginOverlap`
  (params (OverlappedComponent :type "PrimitiveComponent Object Reference") (OtherActor :type "Actor Object Reference") (OtherComp :type "PrimitiveComponent Object Reference") (OtherBodyIndex :type Integer) (bFromSweep :type Boolean) (SweepResult :type "HitResult Structure (by ref)"))
  (if (== OtherActor (`GameplayStatics.GetPlayerCharacter` 0))
    (bind _returnvalue (`KismetSystemLibrary.K2_SetTimerDelegate` (delegate `PushCharacterOut`) 0.01 true))))

(event `PushCharacterOut`
  (bind _returnvalue (`GameplayStatics.GetPlayerCharacter` 0))
  (bind _charactermovement (`Character.CharacterMovement` _returnvalue))
  (bind _returnvalue_x (`KismetMathLibrary.BreakVector` (`KismetMathLibrary.InverseTransformLocation` (`self.GetTransform`) (`self.K2_GetActorLocation` _returnvalue))))
  (bind _velocity_x (`KismetMathLibrary.BreakVector` (`MovementComponent.Velocity` _charactermovement)))
  (bind _returnvalue_2 (`KismetMathLibrary.Abs` (- (.x (`SceneComponent.RelativeLocation` (`self.Box`))) _returnvalue_x)))
  (`KismetSystemLibrary.PrintString` (`KismetStringLibrary.Conv_DoubleToString` _returnvalue_2) true true (struct :`G` 0.66 :`B` 1.0 :`A` 1.0) 0.0)
  (set `MovementComponent.Velocity` (`KismetMathLibrary.MakeVector` _velocity_x) _charactermovement)
  (`CharacterMovementComponent.AddImpulse` _charactermovement (* (`self.GetActorForwardVector`) (* (/ 1.0 _returnvalue_2) 10000.0)) true))

(event `self.Box.OnComponentEndOverlap`
  (params (OverlappedComponent :type "PrimitiveComponent Object Reference") (OtherActor :type "Actor Object Reference") (OtherComp :type "PrimitiveComponent Object Reference") (OtherBodyIndex :type Integer))
  (if (== OtherActor (`GameplayStatics.GetPlayerCharacter` 0))
    (`KismetSystemLibrary.K2_ClearAndInvalidateTimerHandle` (stale `self.Box.OnComponentBeginOverlap` _returnvalue))))

(fn `UserConstructionScript`)